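; Checkpoint marker actor for jump flags in the horse riding demo, cleared when a horse exits its trigger box.
; On BeginPlay it passes its world location to the Marker widget in its widget component.
; When BP_Horse ends overlap, it resets the game mode's LastCheckpoint to None and calls CheckpointClear with its checkpoint number.
; It then hides the trigger and widget and turns off the trigger's overlap events.
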(event OnComponentEndOverlap(TriggerBox)
  (params (OverlappedComponent :type Primitive%20Component%20Object%20Reference) (OtherActor :type Actor%20Object%20Reference) (OtherComp :type Primitive%20Component%20Object%20Reference) (OtherBodyIndex :type Integer))
  (bind _triggerbox (Variables|Default|GetTriggerBox))
  (Utilities|Casting|CastToBP_Horse OtherActor)
  (bind _asbp_horse_riding_demo_game_mode (Utilities|Casting|CastToBP_HorseRidingDemoGameMode (Game|GetGameMode)))
  (Variables|/Game/HorseRidingSystem/DemoScene/BP_HorseRidingDemoGameMode.BP_HorseRidingDemoGameMode_C|Setlast%20checkpoint _asbp_horse_riding_demo_game_mode 0)
  (Default|CallCheckpointClear (Variables|Default|GetCheckpointNumber))
  (Development|SetHiddeninGame _triggerbox true false)
  (Variables|/Script/Engine.PrimitiveComponent|SetbGenerateOverlapEvents _triggerbox false)
  (Rendering|SetVisibility (Variables|Default|Getwidget) false false)
  (Rendering|SetVisibility (Variables|Default|Getwidget) false false))

(event EventBeginPlay
  (bind _asmarker (Utilities|Casting|CastToMarker (UserInterface|GetWidget (Variables|Default|Getwidget))))
  (Variables|/Game/MarkersObjectives/Marker.Marker_C|SetOriginLocation _asmarker (Transformation|GetActorLocation))
  (bind _asmarker_2 (Utilities|Casting|CastToMarker (UserInterface|GetWidget (Variables|Default|Getwidget))))
  (Variables|/Game/MarkersObjectives/Marker.Marker_C|SetOriginLocation _asmarker_2 (Transformation|GetActorLocation)))

(fn ConstructionScript)