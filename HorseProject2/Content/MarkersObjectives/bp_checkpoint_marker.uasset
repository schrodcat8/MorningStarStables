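; Checkpoint marker actor for the horse riding demo, with a widget marker and a box trigger.
; On BeginPlay it passes its world location to the Marker widget as OriginLocation, performing the same cast and assignment twice.
; When a BP_Horse overlaps the box, it sets LastCheckpoint on the demo game mode to None, so the checkpoint does not record itself.
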(event OnComponentBeginOverlap(Box)
  (params (OverlappedComponent :type Primitive%20Component%20Object%20Reference) (OtherActor :type Actor%20Object%20Reference) (OtherComp :type Primitive%20Component%20Object%20Reference) (OtherBodyIndex :type Integer) (bFromSweep :type Boolean) (SweepResult :type Hit%20Result%20Structure%20%28by%20ref%29))
  (Utilities|Casting|CastToBP_Horse OtherActor)
  (bind _asbp_horse_riding_demo_game_mode (Utilities|Casting|CastToBP_HorseRidingDemoGameMode (Game|GetGameMode)))
  (Variables|/Game/HorseRidingSystem/DemoScene/BP_HorseRidingDemoGameMode.BP_HorseRidingDemoGameMode_C|Setlast%20checkpoint _asbp_horse_riding_demo_game_mode 0))

(event EventBeginPlay
  (bind _asmarker (Utilities|Casting|CastToMarker (UserInterface|GetWidget (Variables|Default|GetWidget))))
  (Variables|/Game/MarkersObjectives/Marker.Marker_C|SetOriginLocation _asmarker (Transformation|GetActorLocation))
  (bind _asmarker_2 (Utilities|Casting|CastToMarker (UserInterface|GetWidget (Variables|Default|GetWidget))))
  (Variables|/Game/MarkersObjectives/Marker.Marker_C|SetOriginLocation _asmarker_2 (Transformation|GetActorLocation)))

(fn ConstructionScript)