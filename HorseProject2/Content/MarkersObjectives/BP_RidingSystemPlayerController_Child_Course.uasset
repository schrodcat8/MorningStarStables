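; Player controller for the horse riding course that manages the course HUD, timer and obstacle count.
; On BeginPlay it adds the HUD, caches the course horse pawn and starts a timeline used as the stopwatch.
; Each timeline update converts elapsed time to printed text, while UpdateObstacle advances the obstacle count only when CourseComplete is set.
; Restart, goal updates, time checks and save/load functions are empty stubs.
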(event Custom|Restart)

(event Custom|UpdateObstacle
  ;[1 1 1] Update Obstacles
  (if (Variables|Default|GetCourseComplete)
    (bind _output_get (Variables|ValueVariables|SetActualObstacle (+ (Variables|ValueVariables|GetActualObstacle) 1)))
    (bind _output_get_2 (Variables|TextVariables|SetCurrentObstacleText (Utilities|Text|ToText(Integer) _output_get)))
    (Development|PrintText _output_get_2)))

(event Custom|StartCourseTime
  ;[1 1 1] Course Timer and converts to text
  (bind _time (Timeline|CourseTime Play)
    (:Update
      (bind _output_get (Variables|ValueVariables|SetActualCourseTime _time))
      (bind _output_get_2 (Variables|TextVariables|SetCourseTimeText (Utilities|TimetoText _output_get)))
      (CallFunction|UpdateGoals)
      (Development|PrintText _output_get_2))))

(event Custom|StopCourseTime
  ;[1 1 1] Course Timer and converts to text
  (bind _time (Timeline|CourseTime Stop)
    (:Update
      (bind _output_get (Variables|ValueVariables|SetActualCourseTime _time))
      (bind _output_get_2 (Variables|TextVariables|SetCourseTimeText (Utilities|TimetoText _output_get)))
      (CallFunction|UpdateGoals)
      (Development|PrintText _output_get_2))))

(event EventBeginPlay
  ;[1 1 1] Course HUD
  (bind _returnvalue (UserInterface|CreateWidget "/Game/MarkersObjectives/UI/HUD.HUD_C"))
  (bind _output_get (Variables|Default|SetHUDReference _returnvalue))
  (UserInterface|Viewport|AddtoViewport _output_get 0)
  (bind _asbp_horse_child_course (Utilities|Casting|CastToBP_Horse_Child_Course (Game|Player|GetPlayerPawn 0)))
  (Variables|Default|SetHorseReference _asbp_horse_child_course)
  (CallFunction|StartCourseTime))

(fn ConstructionScript
  (|CallParentFunction))

(fn InitTest)

(fn SaveGameCheck)

(fn SavetheGame)

(fn LoadGame)

(fn CourseTimeCheck)

(fn UpdateGoals)