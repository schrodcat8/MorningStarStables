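; Modular Holsteiner horse demo Blueprint, assembled from a body mesh plus mane, eyelashes, horseshoes and separate tack pieces.
; The construction script applies the mane material to hair and one body slot, a shared material to most tack, and visibility flags per piece.
; Most parts follow the body mesh through leader pose.
; BitVisibility feeds the Headset's propagate-to-children input rather than setting Bit visibility directly.
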(event Collision|EventActorBeginOverlap
  (params (OtherActor :type Actor%20Object%20Reference)))

(event EventTick
  (params (DeltaSeconds :type Float%20%28single-precision%29)))

(fn ConstructionScript
  (bind _mane_colorgen (Variables|Default|GetMane%20ColorGen))
  (Utilities|FlowControl|Sequence
    (:then_0
      (Rendering|Material|SetMaterial (Variables|Default|GetMane) 0 _mane_colorgen)
      (Rendering|Material|SetMaterial (Variables|SkeletalMeshActor|GetSkeletalMeshComponent) 2 _mane_colorgen))
    (:then_1
      (Rendering|Material|SetMaterial (Variables|Default|GetBit) 0 (Variables|TackVisibility|GetTack%20Material)))
    (:then_2
      (Rendering|SetVisibility (Variables|Default|GetHeadset) (Variables|TackVisibility|GetHeadset_Visibility) (Variables|TackVisibility|GetBit%20Visibility))
      (Rendering|SetVisibility (Variables|Default|GetHeadgear%20Fur) (Variables|TackVisibility|GetHeadgear%20Fur%20Visibility) false)
      (Rendering|SetVisibility (Variables|Default|GetPad) (Variables|TackVisibility|GetPad%20Visibility) false)
      (Rendering|SetVisibility (Variables|Default|GetSaddle) (Variables|TackVisibility|GetSaddle%20Visibility) false)
      (Rendering|SetVisibility (Variables|Default|GetHeadwear) (Variables|TackVisibility|GetHeadwear%20Visibility) false)
      (Rendering|SetVisibility (Variables|Default|GetHorseshoes) (Variables|TackVisibility|GetHorseshoes%20Visibility) false)
      (Rendering|SetVisibility (Variables|Default|GetHorse%20boots%20Front) (Variables|TackVisibility|GetFront%20Bandages%20Visibility) false)
      (Rendering|SetVisibility (Variables|Default|GetHorse%20boots%20Rear) (Variables|TackVisibility|GetRear%20Bandages%20Visibility) false)
      (Rendering|SetVisibility (Variables|Default|GetReins) (Variables|TackVisibility|GetReins%20Visibility) false))
    (:then_3
      (Components|SkinnedMesh|SetLeaderPoseComponent (Variables|Default|GetPad) (Variables|SkeletalMeshActor|GetSkeletalMeshComponent) false false))))