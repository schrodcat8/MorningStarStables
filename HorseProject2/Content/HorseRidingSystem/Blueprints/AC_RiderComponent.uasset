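; Rider component for a Character that handles calling, mounting, riding and dismounting horses in multiplayer.
; Mounting walks the rider to the nearest mount point via navmesh or a move fallback; calling sends an available nearby horse or spawns one.
; RepNotify variables swap the mesh to ABP_Rider and feed it riding state.
; Also handles ragdoll with capsule follow, dismount repossession and respawn; legacy and debug input nodes are disabled.
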(event Custom|UpdateCapsuleLocation
  (bind _returnvalue (Utilities|Name|MakeLiteralName "pelvis"))
  (bind _characterowner (Variables|Default|GetCharacterOwner))
  (bind _characterowner_2 (Variables|Default|GetCharacterOwner))
  (bind _capsulecomponent (Variables|/Script/Engine.Character|GetCapsuleComponent _characterowner))
  (bind _mesh (Variables|/Script/Engine.Character|GetMesh _characterowner_2))
  (bind _returnvalue_2 (Transformation|GetSocketLocation _mesh _returnvalue))
  ;[0.2656 0.2656 0.2656] Ragdoll
  ;;[1 1 1] Update Capsule Location on Ragdoll - Client
  (bind (_outhit _returnvalue_3) (Collision|LineTraceByChannel _returnvalue_2 (+ _returnvalue_2 "0,0,-100.000000") "TraceTypeQuery1" false 0 "None"))
  (if _returnvalue_3
    (Variables|Default|SetTargetGroundLocation (.Location (Collision|BreakHitResult _outhit)))
    (else
      (Variables|Default|SetTargetGroundLocation (- (Transformation|GetSocketLocation (Variables|/Script/Engine.Character|GetMesh (Variables|Default|GetCharacterOwner)) _returnvalue) (Variables|Default|GetPelvisOffset)))))
  (Transformation|SetWorldLocation _capsulecomponent (+ (Variables|Default|GetTargetGroundLocation) (Math|Vector|MakeVector 0.0 0.0 (Variables|/Script/Engine.CapsuleComponent|GetCapsuleHalfHeight _capsulecomponent)) "") false false))

(event Custom|ToRagdoll_Server
  ;[0.2656 0.2656 0.2656] Ragdoll
  ;;[0.5284 0.76 1] To Ragdoll - Server
  (Variables|Default|SetIsRagdoll true)
  (CallFunction|ToRagdollMulticast))

(event Custom|RespawnPlayer_Server
  ;[0.4638 0.7403 1] Respawn - Server
  (Variables|Default|SetControllerRef (Pawn|GetController (Variables|Default|GetCharacterOwner)))
  (Actor|DestroyActor (Variables|Default|GetCharacterOwner))
  (Class|GameModeBase|RestartPlayer (Game|GetGameMode) (Variables|Default|GetControllerRef)))

(event Custom|RiderMount_Server
  (params (MountFromRight :type Boolean))
  ;[0.2865 0.2865 0.2865] Rider Mount
  ;;[0.5639 0.7081 1] Rider Mount - Server
  (Variables|Animations|SetUseRiderAnimBP true)
  (Variables|Animations|SetAnims_IsMountAnimationRight MountFromRight)
  (Variables|Animations|SetAnims_IsRiding true)
  (Variables|Animations|SetAnims_MountableActor (Variables|Default|GetMountableActor))
  (CallFunction|RiderMountMulticast))

(event Custom|RiderMount_Multicast
  (bind _characterowner (Variables|Default|GetCharacterOwner))
  ;[0.2865 0.2865 0.2865] Rider Mount
  ;;[1 0.5195 0.4996] Rider Mount - Multicast
  (Collision|SetCollisionEnabled (Variables|/Script/Engine.Character|GetMesh _characterowner) "NoCollision")
  (Pawn|Components|CharacterMovement|SetMovementMode (Variables|/Script/Engine.Character|GetCharacterMovement _characterowner) "MOVE_None" 0))

(event Custom|MoveCameraOnDismountEnd_Owner
  (params (HorseControlRotation :type Rotator))
  ;[0.2604 0.2604 0.2604] Rider Dismount
  ;;[0.4886 1 0.5173] Move Camera on dismount end
  (Pawn|SetControlRotation (Pawn|GetController (Variables|Default|GetCharacterOwner)) HorseControlRotation))

(event Custom|MoveRiderToMountLocation_Multicast
  (params (MountLocation :type Vector) (MountRotation :type Rotator))
  (bind _characterowner (Variables|Default|GetCharacterOwner))
  ;[0.25 0.25 0.25] Rider Move To Mount Location
  ;;[1 0.5424 0.6325] MoveRiderToMountLocation - without navigation - Multicast
  (Development|PrintString "Warning! Mount location isn't inside navigatable area, using MoveComponent instead" true true "(R=1.000000,G=0.652894,B=0.000000,A=1.000000)" 1e+01)
  (Components|MoveComponentTo (Variables|/Script/Engine.Character|GetCapsuleComponent (Variables|Default|GetCharacterOwner)) MountLocation MountRotation false false (/ (Math|Vector|VectorLength (- MountLocation (Transformation|GetActorLocation _characterowner))) (Class|MovementComponent|GetMaxSpeed (Variables|/Script/Engine.Character|GetCharacterMovement _characterowner))) false))

(event Custom|MoveRiderToMountLocationNav_Owner
  (params (MountLocation :type Vector))
  ;[0.25 0.25 0.25] Rider Move To Mount Location
  ;;[0.4279 1 0.4576] MoveRiderToMountLocation - with navigation - Owner
  (AI|Navigation|SimpleMovetoLocation (Pawn|GetController (Variables|Default|GetCharacterOwner)) MountLocation)
  (Variables|Default|SetMovingToMountLocation true))

(event Custom|Set_RiderInMountZone_Server
  (params (Horse :type BP%20Horse%20Object%20Reference) (RiderInMountZone :type Boolean))
  ;[0.25 0.25 0.25] Rider Move To Mount Location
  ;;[0.4223 0.7531 1] Setting Rider Mount flags - Server
  (if (== Horse (Variables|Default|GetMountableActor))
    (Variables|Default|SetRiderInMountZone RiderInMountZone)))

(event Custom|Set_RiderWantsToMount_Server
  (params (RiderWantsToMount :type Boolean))
  ;[0.25 0.25 0.25] Rider Move To Mount Location
  ;;[0.4223 0.7531 1] Setting Rider Mount flags - Server
  (Variables|Default|SetRiderWantsToMount RiderWantsToMount))

(event Custom|Call%20Horse
  (bind _characterowner (Variables|Default|GetCharacterOwner))
  (bind _returnvalue (Transformation|GetActorTransform _characterowner))
  (bind _returnvalue_2 (Transformation|GetActorRightVector _characterowner))
  (bind _capsulecomponent (Variables|/Script/Engine.Character|GetCapsuleComponent _characterowner))
  (bind _returnvalue_3 (Components|Capsule|GetScaledCapsuleHalfHeight _capsulecomponent))
  (bind _returnvalue_4 (* -1.5e+02 _returnvalue_2))
  (bind _returnvalue_5 (- (.location _returnvalue) (Math|Vector|MakeVector (.x _returnvalue_4) (.y _returnvalue_4) _returnvalue_3)))
  (bind (_projectedlocation _returnvalue_6) (AI|Navigation|ProjectPointtoNavigation _returnvalue_5 0 0 "300.000000,300.000000,40.000000"))
  ;[0.4301 0.7076 1] Call Horse - Server
  (bind _outactors (Collision|SphereOverlapActors (Transformation|GetActorLocation (Variables|Default|GetCharacterOwner)) (Variables|Default|GetHorseCallMaxDistance) (Utilities|Array|MakeArray "ObjectTypeQuery3") "/Game/HorseRidingSystem/Blueprints/BP_Horse.BP_Horse_C"))
  (if (> (Utilities|Array|Length _outactors) 0)
    (bind _array_element (Utilities|Array|ForEachLoopwithBreak _outactors :!label _label)
      (:LoopBody
        (bind _asbp_horse (Utilities|Casting|CastToBP_Horse _array_element))
        (bind _canbecalled (Default|CanbeCalled _asbp_horse))
        (if _canbecalled
          (Default|NavigatetoActorServer _asbp_horse (Variables|Default|GetCharacterOwner))
          (Development|PrintString (Utilities|String|Append "Calling " (Utilities|GetDisplayName _asbp_horse)) false)
          (Utilities|FlowControl|Sequence
            (:then_0
              (goto _label Break))
            (:then_1
              (goto _label_2 Close)))
          (else
            (Development|PrintString (Utilities|String|Append (Utilities|GetDisplayName _asbp_horse) " can't be called") false true "(R=1.000000,G=0.954167,B=0.165041,A=1.000000)" 4.0)
            (goto _label_2 Open))))
      (:Completed
        (Utilities|FlowControl|Gate false :!label _label_2
          (:Exit
            _)))))
  (Development|PrintString "No horses in call range, spawning one..." true true "(R=0.340677,G=1.000000,B=0.062211,A=1.000000)" 8.0)
  (if _returnvalue_6
    (bind _returnvalue_7 (Game|SpawnActorfromClass "/Game/HorseRidingSystem/Blueprints/BP_Horse.BP_Horse_C" (Math|Transform|MakeTransform _projectedlocation (.rotation _returnvalue) "1.000000,1.000000,1.000000") "AdjustIfPossibleButDontSpawnIfColliding" 0 0))
    (Pawn|SpawnDefaultController _returnvalue_7)
    (Variables|/Game/HorseRidingSystem/Blueprints/BP_Horse.BP_Horse_C|SetCachedRoamingController _returnvalue_7 (Pawn|GetController _returnvalue_7))
    (Development|PrintString (Utilities|String|Append "Spawned " (Utilities|GetDisplayName _returnvalue_7)) false)
    (else
      (Development|PrintString "Can't spawn new horse" true true "(R=1.000000,G=0.000000,B=0.057610,A=1.000000)" 5.0))))

(event Custom|ToRagdoll_Multicast
  (bind _characterowner (Variables|Default|GetCharacterOwner))
  (bind _characterowner_2 (Variables|Default|GetCharacterOwner))
  (bind _mesh (Variables|/Script/Engine.Character|GetMesh _characterowner))
  ;[0.2656 0.2656 0.2656] Ragdoll
  ;;[1 0.4258 0.4059] To Ragdoll - Multicast
  (Collision|SetCollisionEnabled _mesh "QueryAndPhysics")
  (Class|SkeletalMeshComponent|SetAllBodiesBelowSimulatePhysics _mesh (Utilities|Name|MakeLiteralName "pelvis") true true)
  (Pawn|Components|CharacterMovement|DisableMovement (Variables|/Script/Engine.Character|GetCharacterMovement _characterowner_2))
  (Collision|SetCollisionEnabled (Variables|/Script/Engine.Character|GetCapsuleComponent _characterowner_2) "NoCollision")
  (Development|PrintString "Rider Ragdoll" false))

(event Custom|MountRider_Client
  ;[0.25 0.25 0.25] Rider Move To Mount Location
  ;;[1 1 1] MountRider Action - Client
  (CallFunction|MountRiderServer))

(event Custom|MountRider_Server
  (bind _mountableactor (Variables|Default|GetMountableActor))
  ;[0.25 0.25 0.25] Rider Move To Mount Location
  ;;[0.4861 0.8484 1] MountRider Action - Server
  (Utilities|IsValid (Variables|Animations|GetRiderAnims)
    (:Is%20Valid
      (if (Variables|Animations|GetAnims_IsRiding)
        (Development|PrintString "RiderAnims is still riding" true true "(R=1.000000,G=0.000000,B=0.047706,A=1.000000)")
        (else
          (Utilities|IsValid (Variables|Default|GetMountableActor) :!label _label
            (:Is%20Valid
              (Class|BIHorse|MountHorse(Message) _mountableactor (Variables|Default|GetCharacterOwner))
              (bind (_isright _mountposition _mountrotation) (Class|BIHorse|FindNearestMountLocation(Message) _mountableactor))
              (if (.ReturnValue (AI|Navigation|ProjectPointtoNavigation _mountposition 0 0 "0, 0, 0")) ; Check if mount location is iside the navigation area
                (CallFunction|MoveRidertoMountLocationNavOwner (.ProjectedLocation (AI|Navigation|ProjectPointtoNavigation _mountposition 0 0 "0, 0, 0")))
                (else
                  (CallFunction|MoveRidertoMountLocationMulticast _mountposition _mountrotation))))
            (:Is%20Not%20Valid
              (Development|PrintString "Mountable actor is not valid" true true "(R=1.000000,G=0.000000,B=0.127628,A=1.000000)"))))))
    (:Is%20Not%20Valid
      (goto _label))))

(event Custom|StopMovingToMountLocation
  ;[0.25 0.25 0.25] Rider Move To Mount Location
  ;;[1 1 1] Stop auto move to mount position on any movement input - Client
  (if (Variables|Default|GetMovingToMountLocation)
    (AI|Navigation|StopMovement (Pawn|GetController (Variables|Default|GetCharacterOwner)))
    (Variables|Default|SetMovingToMountLocation false)
    (CallFunction|SetRiderWantstoMountServer false)
    (Development|PrintString "Stop Movement" false)))

(event Custom|RiderFall_Server
  ;[0.2656 0.2656 0.2656] Ragdoll
  ;;[0.4696 0.8276 1] Rider Fall event (Rider Ragdoll Start)
  (Variables|Animations|SetAnims_IsRagdoll true))

(event EventRiderMount
  (params (MountFromRight :type Boolean))
  ;[0.2865 0.2865 0.2865] Rider Mount
  ;;[1 1 1] Rider Mount event (Rider Mounting Start) - Client
  (CallFunction|RiderMountServer MountFromRight))

(event EventResetMountableHorse
  (params (MountableHorse :type BP%20Horse%20Object%20Reference))
  ;[0.3125 0.3125 0.3125] Horse Left
  ;;[0.3421 0.7443 1] Horse Left  Event - Reset Mountable Horse - Server
  (if (== MountableHorse (Variables|Default|GetMountableActor))
    (Variables|Default|SetMountableActor 0)
    (Development|PrintString "Same horse, resetting mountable horse" false true "(R=0.041467,G=1.000000,B=0.000000,A=1.000000)")
    (else
      (Development|PrintString "Other horse, ignoring horse reset" false true "(R=1.000000,G=0.804508,B=0.000000,A=1.000000)"))))

(event EventTick
  (params (DeltaSeconds :type Float%20%28single-precision%29))
  ;[1 1 1] Tick
  (if (Variables|Default|GetIsRagdoll)
    (CallFunction|UpdateCapsuleLocation)))

(event EventRiderDismountEnd
  (bind _mountableactor (Variables|Default|GetMountableActor))
  ;[0.2604 0.2604 0.2604] Rider Dismount
  ;;[0.4362 0.8488 1] RiderDismount End - Server (Called from Server)
  (Variables|Animations|SetAnims_MountableActor 0)
  (Variables|Default|SetHorseControlRotation (Pawn|GetControlRotation _mountableactor :!class /Script/Engine.Pawn))
  (Pawn|Possess (Pawn|GetController _mountableactor) (Variables|Default|GetCharacterOwner))
  (CallFunction|MoveCameraonDismountEndOwner (Variables|Default|GetHorseControlRotation))
  (Default|ShowMountUIOwner (Variables|Default|GetMountableActor) (Variables|Default|GetCharacterOwner)) ; Show Mount Tooltip
  (Utilities|FlowControl|DelayUntilNextTick) ; UE crashes without this
  (Variables|Animations|SetUseRiderAnimBP false))

(event EventBeginPlay
  ;[0.05098 0.05098 0.05098] Begin Play
  (Utilities|FlowControl|Sequence
    (:then_0
      ;;[1 1 1] Cache Components
      (bind _ascharacter (Utilities|Casting|CastToCharacter (Components|GetOwner))
        (:then
          (Variables|Default|SetCharacterOwner _ascharacter)
          (Variables|Default|SetCharacterCamera (Actor|GetComponentbyClass (Variables|Default|GetCharacterOwner) "/Script/Engine.CameraComponent")))
        (:CastFailed
          (Development|PrintString "Character owner cast failed!" true true "(R=1.000000,G=0.000000,B=0.096547,A=1.000000)"))))
    (:then_1
      ;;[1 1 1] Set Pelvis Offset for Ragdoll
      (Variables|Default|SetPelvisOffset (- (Transformation|GetSocketLocation (Variables|/Script/Engine.Character|GetMesh (Variables|Default|GetCharacterOwner)) (Utilities|Name|MakeLiteralName "pelvis")) (Transformation|GetSocketLocation (Variables|/Script/Engine.Character|GetMesh (Variables|Default|GetCharacterOwner)) (Utilities|Name|MakeLiteralName "root")))))
    (:then_2
      ;;[1 1 1] Set Enhanced Input
      (Variables|Default|SetUseEnhancedInput (Utilities|IsValid (Actor|GetComponentbyClass (Variables|Default|GetCharacterOwner) 0))))))

(event EventRiderDismount
  (params (DismountToRight :type Boolean))
  ;[0.2604 0.2604 0.2604] Rider Dismount
  ;;[0.4294 0.7963 1] Rider Dismount event (Rider Dismounting Start) - Server (Called from server)
  (Variables|Animations|SetAnims_IsMountAnimationRight DismountToRight)
  (Variables|Animations|SetAnims_IsRiding false))

(event EventSetMountableHorse
  (params (MountableHorse :type BP%20Horse%20Object%20Reference))
  ;[0.2344 0.2344 0.2344] Horse Approach
  ;;[0.4428 0.8068 1] Horse approach Event - Set Mountable Actor - Server
  (bind _output_get (Variables|Default|SetMountableActor MountableHorse))
  (Development|PrintString (Utilities|String|Append "Mountable actor set: " (Utilities|GetDisplayName _output_get)) false true "(R=1.000000,G=0.919933,B=0.000000,A=1.000000)" 5.0))

(event Input|ActionEvents|InputActionInteract
  (params (Key :type Key%20Structure :default "None"))
  ;[1 0.5541 0.945] Legacy Input: To Use - download the Input Config file from the asset description and enable these nodes (Turn on "Allow Explicit Impure Node Disabling" in Editor Settings to allow enabling/disabling nodes). Also check BP_Horse for Legacy input section. See more in the Manual
  ;;[0.9085 0.4927 1] Interact - Legacy Input
  (:Pressed
    (Utilities|FlowControl|DoOnce false :!label _label
      (:Completed
        (if (Variables|Default|GetUseEnhancedInput)
          (Development|PrintString "Using Enhanced Input" false)
          (else
            (CallFunction|MountRiderClient))))))
  (:Released
    (goto _label Reset)))

(event Input|ActionEvents|InputActionHorseDropDead
  (params (Key :type Key%20Structure :default "None"))
  ;[0.2656 0.2656 0.2656] Debug - Turned Off
  ;;[1 0.828 0.4247] DropDead Action - Debug
  (:Pressed
    (Utilities|FlowControl|DoOnce false :!label _label
      (:Completed
        (if (not (Variables|Default|GetIsRagdoll))
          (CallFunction|ToRagdollServer)))))
  (:Released
    (goto _label Reset)))

(event Input|ActionEvents|InputActionRespawn
  (params (Key :type Key%20Structure :default "None"))
  ;[0.2656 0.2656 0.2656] Debug - Turned Off
  ;;[1 0.9157 0.4371] Respawn - Debug
  (:Pressed
    (Utilities|FlowControl|DoOnce false :!label _label
      (:Completed
        (CallFunction|RespawnPlayerClient))))
  (:Released
    (goto _label Reset)))

(event Input|AxisEvents|InputAxisMoveForward/Backward
  (params (AxisValue :type Float%20%28single-precision%29))
  ;[1 0.5541 0.945] Legacy Input: To Use - download the Input Config file from the asset description and enable these nodes (Turn on "Allow Explicit Impure Node Disabling" in Editor Settings to allow enabling/disabling nodes). Also check BP_Horse for Legacy input section. See more in the Manual
  ;;[1 0.4562 0.9417] Stop Moving to Mount Location - Legacy Input
  (if (or (!= AxisValue 0.0) (!= (stale Input|AxisEvents|InputAxisMoveRight/Left AxisValue) 0.0))
    (CallFunction|StopMovingtoMountLocation)))

(event Input|AxisEvents|InputAxisMoveRight/Left
  (params (AxisValue :type Float%20%28single-precision%29))
  ;[1 0.5541 0.945] Legacy Input: To Use - download the Input Config file from the asset description and enable these nodes (Turn on "Allow Explicit Impure Node Disabling" in Editor Settings to allow enabling/disabling nodes). Also check BP_Horse for Legacy input section. See more in the Manual
  ;;[1 0.4562 0.9417] Stop Moving to Mount Location - Legacy Input
  (if (or (!= (stale Input|AxisEvents|InputAxisMoveForward/Backward AxisValue) 0.0) (!= AxisValue 0.0))
    (CallFunction|StopMovingtoMountLocation)))

(fn SetHorseJump
  (params (Jump :type E_HorseJumps%20Enum :default "NewEnumerator4"))
  (Variables|Animations|SetAnims_HorseJump Jump))

(fn SpurHorse
  (Default|SpurHorse (Variables|Animations|GetRiderAnims)))

(fn OnRepAnimsIsRiding
  (Utilities|IsValid (Variables|Animations|GetRiderAnims)
    (:Is%20Valid
      (Variables|/Game/HorseRidingSystem/Blueprints/AnimationBlueprints/ABP_Rider.ABP_Rider_C|SetisRiding (Variables|Animations|GetRiderAnims) (Variables|Animations|GetAnims_IsRiding))
      (Development|PrintString "Anims_isriding set" false true "(R=1.000000,G=0.764541,B=0.000000,A=1.000000)" 1e+01))
    (:Is%20Not%20Valid
      (Development|PrintString "ABP RIDER not valid - isRiding" true true "(R=1.000000,G=0.065008,B=0.000000,A=1.000000)" 1e+01))))

(fn OnRepUseRiderAnimBP
  (bind _characterowner (Variables|Default|GetCharacterOwner))
  (bind _mesh (Variables|/Script/Engine.Character|GetMesh _characterowner))
  (if (Variables|Animations|GetUseRiderAnimBP)
    (Variables|Default|SetCachedAnimInstanceClass (Utilities|GetClass (Components|SkeletalMesh|GetAnimInstance _mesh)))
    (Class|SkeletalMeshComponent|SetAnimClass _mesh "/Game/HorseRidingSystem/Blueprints/AnimationBlueprints/ABP_Rider.ABP_Rider_C")
    (bind _asabp_rider (Utilities|Casting|CastToABP_Rider (Components|SkeletalMesh|GetAnimInstance (Variables|/Script/Engine.Character|GetMesh (Variables|Default|GetCharacterOwner))))
      (:then
        (Variables|Animations|SetRiderAnims _asabp_rider))
      (:CastFailed
        (Development|PrintString "Ride Anims Cast Failed" true true "(R=1.000000,G=0.000000,B=0.034335,A=1.000000)" 4.0)))
    (else
      (Class|SkeletalMeshComponent|SetAnimClass (Variables|/Script/Engine.Character|GetMesh (Variables|Default|GetCharacterOwner)) (Variables|Default|GetCachedAnimInstanceClass))
      (Variables|Animations|SetRiderAnims 0))))

(fn OnRepAnimsIsMountAnimationRight
  (Utilities|IsValid (Variables|Animations|GetRiderAnims)
    (:Is%20Valid
      (Variables|/Game/HorseRidingSystem/Blueprints/AnimationBlueprints/ABP_Rider.ABP_Rider_C|SetIsMountAnimationRight (Variables|Animations|GetRiderAnims) (Variables|Animations|GetAnims_IsMountAnimationRight))
      (Development|PrintString "Anims_ismountanimationright set" false true "(R=1.000000,G=0.764541,B=0.000000,A=1.000000)" 1e+01))
    (:Is%20Not%20Valid
      (Development|PrintString "ABP RIDER not valid - isMountAnimRight" true true "(R=1.000000,G=0.065008,B=0.000000,A=1.000000)" 1e+01))))

(fn OnRepAnimsMountableActor
  (Utilities|IsValid (Variables|Animations|GetRiderAnims)
    (:Is%20Valid
      (Variables|/Game/HorseRidingSystem/Blueprints/AnimationBlueprints/ABP_Rider.ABP_Rider_C|SetMountableActor (Variables|Animations|GetRiderAnims) (Variables|Animations|GetAnims_MountableActor))
      (Development|PrintString "Anims_mountableActor set" false true "(R=1.000000,G=0.764541,B=0.000000,A=1.000000)" 1e+01))
    (:Is%20Not%20Valid
      (Development|PrintString "ABP RIDER not valid - MountableActor" true true "(R=1.000000,G=0.065008,B=0.000000,A=1.000000)" 1e+01))))

(fn OnRepAnimsHorseCurrentAction
  (Utilities|IsValid (Variables|Animations|GetRiderAnims)
    (:Is%20Valid
      (Variables|/Game/HorseRidingSystem/Blueprints/AnimationBlueprints/ABP_Rider.ABP_Rider_C|SetHorseCurrentAction (Variables|Animations|GetRiderAnims) (Variables|Animations|GetAnims_HorseCurrentAction))
      (Development|PrintString "Anims_horseCurrentAction set" false true "(R=1.000000,G=0.764541,B=0.000000,A=1.000000)" 1e+01))
    (:Is%20Not%20Valid
      (Development|PrintString "ABP RIDER not valid - horse current action" true true "(R=1.000000,G=0.065008,B=0.000000,A=1.000000)" 1e+01))))

(fn SetHorseAction
  (params (HorseAction :type E_HorseActions%20Enum :default "NewEnumerator2"))
  (Variables|Animations|SetAnims_HorseCurrentAction HorseAction))

(fn OnRepAnimsIsRagdoll
  (Utilities|IsValid (Variables|Animations|GetRiderAnims)
    (:Is%20Valid
      (Variables|/Game/HorseRidingSystem/Blueprints/AnimationBlueprints/ABP_Rider.ABP_Rider_C|SetIsRagdoll (Variables|Animations|GetRiderAnims) (Variables|Animations|GetAnims_IsRagdoll)))
    (:Is%20Not%20Valid
      (Development|PrintString "ABP RIDER not valid - isRagdoll" true true "(R=1.000000,G=0.065008,B=0.000000,A=1.000000)" 1e+01))))

(fn OnRepAnimsHorseJump
  (Utilities|IsValid (Variables|Animations|GetRiderAnims)
    (:Is%20Valid
      (Variables|/Game/HorseRidingSystem/Blueprints/AnimationBlueprints/ABP_Rider.ABP_Rider_C|SetHorseCurrentJump (Variables|Animations|GetRiderAnims) (Variables|Animations|GetAnims_HorseJump)))
    (:Is%20Not%20Valid
      (Development|PrintString "ABP RIDER not valid - Jump" true true "(R=1.000000,G=0.065008,B=0.000000,A=1.000000)" 1e+01))))

(fn MoveCamera
  (params (Location :type Vector :default "0, 0, 0") (Rotation :type Rotator :default "0, 0, 0")))

(fn IsPlayer
  (return (Pawn|IsPlayerControlled (Variables|Default|GetCharacterOwner))))