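; Blueprint Interface for a rideable horse in the horse riding system, declaring functions only, with no logic.
; It covers mounting and rider mount/dismount, idle-gallop transitions, jump, fall, water entry and exit, and death.
; Query functions expose speed, root rotation, the nearest mount location with its side, and saddle, rider feet and reins socket transforms.
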(fn MountHorse
  (params (Rider :type Character%20Object%20Reference)))

(fn GetHorseSpeed
  (return 0.0))

(fn IdletoGallop)

(fn GalloptoIdle)

(fn EnterWater)

(fn ExitWater)

(fn RiderMounted)

(fn RiderDismounted)

(fn JumpStart)

(fn JumpEnd)

(fn FallStart)

(fn GetRiderFeetTransform
  (return "" ""))

(fn FindNearestMountLocation
  (return false "0, 0, 0" "0, 0, 0"))

(fn GetHorseSaddleTransform
  (return ""))

(fn Die)

(fn GetReinsSocketsTransform
  (return "" "" "" "" "" "" ""))

(fn GetRootRotation
  (return "0, 0, 0"))