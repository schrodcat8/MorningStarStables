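; Actor component that handles Enhanced Input for a rider character in the horse riding system.
; On BeginPlay it adds the rider mapping context to player 0, caches the owner's rider component and removes the context when the character is destroyed.
; Input actions drive character movement, camera and jump, and forward mount and horse-call requests to the rider component, firing once per press.
; Moving also cancels any move to the mount location.
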(event Custom|RemoveRiderMappingContext
  (params (DestroyedActor :type Actor%20Object%20Reference))
  (bind _returnvalue (Game|GetPlayerController 0))
  (bind _returnvalue_2 (PlayerController|LocalPlayerSubsystems|GetEnhancedInputLocalPlayerSubsystem _returnvalue))
  ;[1 1 1] BeginPlay
  (Utilities|IsValid _returnvalue_2
    (:Is%20Valid
      (Input|RemoveMappingContext _returnvalue_2 "/Game/HorseRidingSystem/EnhancedInput/Rider/IMC_Rider.IMC_Rider" "(bIgnoreAllPressedKeysUntilRelease=True,bForceImmediately=False)")
      (Development|PrintString "Rider Input Removed" false))))

(event Input|EnhancedActionEvents|EnhancedInputActionIA_MoveRider
  (params (ActionValue :type Vector%202D%20Structure) (ElapsedSeconds :type Float%20%28double-precision%29) (TriggeredSeconds :type Float%20%28double-precision%29) (InputAction :type Input%20Action%20Object%20Reference :default "/Game/HorseRidingSystem/EnhancedInput/Rider/IA_MoveRider.IA_MoveRider"))
  (bind _ridercomponent (Variables|Default|GetRiderComponent))
  (bind _characterowner (Variables|/Game/HorseRidingSystem/Blueprints/AC_RiderComponent.AC_RiderComponent_C|GetCharacterOwner _ridercomponent))
  (bind _returnvalue (Pawn|GetControlRotation _characterowner :!class /Script/Engine.Pawn))
  ;[1 1 1] Move Action
  (:Triggered
    (Pawn|Input|AddMovementInput (Variables|/Game/HorseRidingSystem/Blueprints/AC_RiderComponent.AC_RiderComponent_C|GetCharacterOwner (Variables|Default|GetRiderComponent)) (Math|Vector|GetRightVector (Math|Rotator|MakeRotator (.roll _returnvalue) 0.0 (.yaw _returnvalue))) (.x ActionValue) false)
    (Pawn|Input|AddMovementInput (Variables|/Game/HorseRidingSystem/Blueprints/AC_RiderComponent.AC_RiderComponent_C|GetCharacterOwner (Variables|Default|GetRiderComponent)) (Math|Vector|GetForwardVector (Math|Rotator|MakeRotator 0.0 0.0 (.yaw (Pawn|GetControlRotation _characterowner :!class /Script/Engine.Pawn)))) (.y ActionValue) false)
    (Default|StopMovingtoMountLocation (Variables|Default|GetRiderComponent))))

(event Input|EnhancedActionEvents|EnhancedInputActionIA_InteractRider
  (params (ActionValue :type Boolean) (ElapsedSeconds :type Float%20%28double-precision%29) (TriggeredSeconds :type Float%20%28double-precision%29) (InputAction :type Input%20Action%20Object%20Reference :default "/Game/HorseRidingSystem/EnhancedInput/Rider/IA_InteractRider.IA_InteractRider"))
  ;[1 1 1] InteractRider Action
  (:Triggered
    (Utilities|FlowControl|DoOnce false :!label _label
      (:Completed
        (Default|MountRiderClient (Variables|Default|GetRiderComponent)))))
  (:Completed
    (goto _label Reset)))

(event Input|EnhancedActionEvents|EnhancedInputActionIA_CallHorseRider
  (params (ActionValue :type Boolean) (ElapsedSeconds :type Float%20%28double-precision%29) (TriggeredSeconds :type Float%20%28double-precision%29) (InputAction :type Input%20Action%20Object%20Reference :default "/Game/HorseRidingSystem/EnhancedInput/Rider/IA_CallHorseRider.IA_CallHorseRider"))
  ;[1 1 1] Call Horse Action
  (:Triggered
    (Utilities|FlowControl|DoOnce false :!label _label
      (:Completed
        (Default|CallHorse (Variables|Default|GetRiderComponent)))))
  (:Completed
    (goto _label Reset)))

(event Input|EnhancedActionEvents|EnhancedInputActionIA_RotateCamera
  (params (ActionValue :type Vector%202D%20Structure) (ElapsedSeconds :type Float%20%28double-precision%29) (TriggeredSeconds :type Float%20%28double-precision%29) (InputAction :type Input%20Action%20Object%20Reference :default "/Game/HorseRidingSystem/EnhancedInput/Common/IA_RotateCamera.IA_RotateCamera"))
  (bind _ridercomponent (Variables|Default|GetRiderComponent))
  (bind _characterowner (Variables|/Game/HorseRidingSystem/Blueprints/AC_RiderComponent.AC_RiderComponent_C|GetCharacterOwner _ridercomponent))
  ;[1 1 1] Rotate Camera Action
  (:Triggered
    (Pawn|Input|AddControllerYawInput _characterowner (.x ActionValue))
    (Pawn|Input|AddControllerPitchInput _characterowner (.y ActionValue))))

(event Input|EnhancedActionEvents|EnhancedInputActionIA_Jump
  (params (ActionValue :type Boolean) (ElapsedSeconds :type Float%20%28double-precision%29) (TriggeredSeconds :type Float%20%28double-precision%29) (InputAction :type Input%20Action%20Object%20Reference :default "/Game/HorseRidingSystem/EnhancedInput/Common/IA_Jump.IA_Jump"))
  (bind _ridercomponent (Variables|Default|GetRiderComponent))
  (bind _characterowner (Variables|/Game/HorseRidingSystem/Blueprints/AC_RiderComponent.AC_RiderComponent_C|GetCharacterOwner _ridercomponent))
  ;[1 1 1] Jump Action
  (:Triggered
    (Character|Jump _characterowner))
  (:Completed
    (Character|StopJumping _characterowner)))

(event EventBeginPlay
  (bind _returnvalue (Game|GetPlayerController 0))
  (bind _returnvalue_2 (Components|GetOwner))
  (bind _returnvalue_3 (Actor|GetComponentbyClass _returnvalue_2 "/Game/HorseRidingSystem/Blueprints/AC_RiderComponent.AC_RiderComponent_C"))
  (bind _returnvalue_4 (PlayerController|LocalPlayerSubsystems|GetEnhancedInputLocalPlayerSubsystem _returnvalue))
  ;[1 1 1] BeginPlay
  (Utilities|FlowControl|Sequence
    (:then_0
      (Utilities|IsValid _returnvalue_4
        (:Is%20Valid
          (Input|AddMappingContext _returnvalue_4 "/Game/HorseRidingSystem/EnhancedInput/Rider/IMC_Rider.IMC_Rider" 0 "(bIgnoreAllPressedKeysUntilRelease=True,bForceImmediately=False)")
          (Development|PrintString "Rider Input Added" false true "(R=0.000000,G=0.660000,B=1.000000,A=1.000000)" 5.0))))
    (:then_1
      (Utilities|IsValid _returnvalue_3
        (:Is%20Valid
          (bind _output_get (Variables|Default|SetRiderComponent _returnvalue_3))
          (Game|BindEventtoOnDestroyed (Variables|/Game/HorseRidingSystem/Blueprints/AC_RiderComponent.AC_RiderComponent_C|GetCharacterOwner _output_get) (delegate Custom|RemoveRiderMappingContext)))
        (:Is%20Not%20Valid
          (Development|PrintString "Rider Component not found" true true "(R=1.000000,G=0.000000,B=0.066670,A=1.000000)"))))))